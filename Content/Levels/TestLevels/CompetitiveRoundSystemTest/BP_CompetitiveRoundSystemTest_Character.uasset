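; Test character for the competitive round system test level, with basic movement, an attack key and a team name tag.
; WASD key events build a world-space move vector that Tick feeds into movement input, and K forwards Attack to the test player controller.
; The name tag widget shows the Team value at BeginPlay and updates on team changes.
; A LineTrace helper returns a debug-drawn visibility trace along fixed world +X from the capsule.
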(event Custom|CustomEvent
  (params (Team :type ETeam%20Enum :default "None"))
  (Rendering|Components|TextRender|SetText (Variables|/Game/Levels/TestLevels/CompetitiveRoundSystemTest/BP_CompetitiveRoundSystemTest_PlayerTeamTag.BP_CompetitiveRoundSystemTest_PlayerTeamTag_C|GetPlayerTeamText (.AsBP%20Competitive%20Round%20System%20Test%20Player%20Team%20Tag (Utilities|Casting|CastToBP_CompetitiveRoundSystemTest_PlayerTeamTag (UserInterface|GetWidget (Variables|Default|GetPlayerNameTag))))) (Utilities|Text|ToText(String) (Utilities|String|EnumtoString Team))))

(event EventTick
  (params (DeltaSeconds :type Float%20%28single-precision%29))
  (Pawn|Input|AddMovementInput (Variables|Default|GetMove%20Vector) 1.0 false))

(event EventBeginPlay
  (bind _team (Variables|Default|GetTeam))
  (bind _returnvalue (Class|TeamComponent|GetTeam _team))
  (bind _returnvalue_2 (Utilities|String|EnumtoString _returnvalue))
  (bind _returnvalue_3 (Utilities|Text|ToText(String) _returnvalue_2))
  (Class|TeamComponent|BindonTeamChanged (Variables|Default|GetTeam) (delegate Custom|CustomEvent))
  (Rendering|Components|TextRender|SetText (Variables|/Game/Levels/TestLevels/CompetitiveRoundSystemTest/BP_CompetitiveRoundSystemTest_PlayerTeamTag.BP_CompetitiveRoundSystemTest_PlayerTeamTag_C|GetPlayerTeamText (.AsBP%20Competitive%20Round%20System%20Test%20Player%20Team%20Tag (Utilities|Casting|CastToBP_CompetitiveRoundSystemTest_PlayerTeamTag (UserInterface|GetWidget (Variables|Default|GetPlayerNameTag))))) _returnvalue_3)
  (Development|PrintText _returnvalue_3))

(event Input|KeyboardEvents|W
  (params (Key :type Key%20Structure :default "None"))
  (:Pressed
    (Variables|Default|SetMove%20Vector (+ (Variables|Default|GetMove%20Vector) "1.000000,0.000000,0.000000")))
  (:Released
    (Variables|Default|SetMove%20Vector (- (Variables|Default|GetMove%20Vector) "1.000000,0.000000,0.000000"))))

(event Input|KeyboardEvents|S
  (params (Key :type Key%20Structure :default "None"))
  (:Pressed
    (Variables|Default|SetMove%20Vector (+ (Variables|Default|GetMove%20Vector) "-1.000000,0.000000,0.000000")))
  (:Released
    (Variables|Default|SetMove%20Vector (- (Variables|Default|GetMove%20Vector) "-1.000000,0.000000,0.000000"))))

(event Input|KeyboardEvents|A
  (params (Key :type Key%20Structure :default "None"))
  (:Pressed
    (Variables|Default|SetMove%20Vector (+ (Variables|Default|GetMove%20Vector) "0.000000,-1.000000,0.000000")))
  (:Released
    (Variables|Default|SetMove%20Vector (- (Variables|Default|GetMove%20Vector) "0.000000,-1.000000,0.000000"))))

(event Input|KeyboardEvents|D
  (params (Key :type Key%20Structure :default "None"))
  (:Pressed
    (Variables|Default|SetMove%20Vector (+ (Variables|Default|GetMove%20Vector) "0.000000,1.000000,0.000000")))
  (:Released
    (Variables|Default|SetMove%20Vector (- (Variables|Default|GetMove%20Vector) "0.000000,1.000000,0.000000"))))

(event Input|KeyboardEvents|K
  (params (Key :type Key%20Structure :default "None"))
  (:Pressed
    (Default|Attack (.AsBP%20Competitive%20Round%20System%20Test%20Player%20Controller (Utilities|Casting|CastToBP_CompetitiveRoundSystemTest_PlayerController (Pawn|GetController))))))

(fn ConstructionScript)

(fn LineTrace
  (bind _capsulecomponent (Variables|Default|GetCapsuleComponent))
  (bind _returnvalue (Transformation|GetWorldLocation _capsulecomponent))
  (bind (_outhit _returnvalue_2) (Collision|LineTraceByChannel _returnvalue (+ _returnvalue "300.000000,0.000000,0.000000") "TraceTypeQuery1" false 0 "Persistent"))
  (return _outhit _returnvalue_2))