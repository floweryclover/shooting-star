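; Player controller for the competitive round system test level, linking players to teams, the test HUD and attacks.
; On possession it copies its team component's team onto the test character, and on local controllers it creates and shows the HUD at begin play.
; Its Attack event line-traces from the controlled character and passes any hit actor to the test game mode's Attack as the attackee.
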(event Custom|Attack
  (bind _returnvalue (Pawn|GetControlledPawn))
  (bind _asbp_competitive_round_system_test_character (Utilities|Casting|CastToBP_CompetitiveRoundSystemTest_Character _returnvalue))
  (bind (_outhit _returnvalue_2) (Default|LineTrace _asbp_competitive_round_system_test_character))
  (if _returnvalue_2
    (Default|Attack (.AsBP%20Competitive%20Round%20System%20Test%20Game%20Mode (Utilities|Casting|CastToBP_CompetitiveRoundSystemTest_GameMode (Game|GetGameMode))) _returnvalue (.HitActor (Collision|BreakHitResult _outhit)))))

(event EventBeginPlay
  (if (Pawn|IsLocalPlayerController)
    (bind _returnvalue (UserInterface|CreateWidget "/Game/Levels/TestLevels/CompetitiveRoundSystemTest/BP_CompetitiveRoundSystemTest_HUD.BP_CompetitiveRoundSystemTest_HUD_C"))
    (bind _output_get (Variables|Default|SetHUD _returnvalue))
    (UserInterface|Viewport|AddtoViewport _output_get 0)))

(event EventPossess
  (params (PossessedPawn :type Pawn%20Object%20Reference))
  (Class|TeamComponent|SetTeam (Variables|/Game/Levels/TestLevels/CompetitiveRoundSystemTest/BP_CompetitiveRoundSystemTest_Character.BP_CompetitiveRoundSystemTest_Character_C|GetTeam (.AsBP%20Competitive%20Round%20System%20Test%20Character (Utilities|Casting|CastToBP_CompetitiveRoundSystemTest_Character PossessedPawn))) (Class|TeamComponent|GetTeam (Variables|Default|GetTeamComponent))))

(fn ConstructionScript)