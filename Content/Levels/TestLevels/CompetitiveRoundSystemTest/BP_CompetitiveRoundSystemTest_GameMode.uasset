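; Test-level game mode for the competitive round system, handling scoring when one actor attacks another.
; The Attack event only counts during the Game phase of its CompetitiveSystemComponent.
; It reads both actors' TeamComponents and, when they are on different, assigned teams, awards fixed round score to the attacker's team.
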(event Custom|Attack
  (params (Attacker :type Actor%20Object%20Reference) (Attackee :type Actor%20Object%20Reference))
  (bind _returnvalue (Actor|GetComponentbyClass Attackee "/Script/ShootingStar.TeamComponent"))
  (bind _returnvalue_2 (Actor|GetComponentbyClass Attacker "/Script/ShootingStar.TeamComponent"))
  (bind _returnvalue_3 (Class|TeamComponent|GetTeam _returnvalue_2))
  (bind _returnvalue_4 (Class|TeamComponent|GetTeam _returnvalue))
  (if (Utilities|Enum|Equal(Enum) (Variables|/Script/ShootingStar.CompetitiveSystemComponent|GetCurrentPhase (Variables|Default|GetCompetitiveSystemComponent)) "Game")
    (Utilities|IsValid _returnvalue_2
      (:Is%20Valid
        (Utilities|IsValid _returnvalue
          (:Is%20Valid
            (if (and (Utilities|Enum|NotEqual(Enum) _returnvalue_3 _returnvalue_4) (and (Utilities|Enum|NotEqual(Enum) _returnvalue_3 "None") (Utilities|Enum|NotEqual(Enum) _returnvalue_4 "None")))
              (Class|CompetitiveSystemComponent|GiveRoundScoreforTeam (Variables|Default|GetCompetitiveSystemComponent) _returnvalue_3 10))))))))

(event EventTick
  (params (DeltaSeconds :type Float%20%28single-precision%29)))

(fn ConstructionScript)