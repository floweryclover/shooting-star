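; BP_CompetitivePlayerCharacter is a player character that displays its player name on an attached name tag widget.
; On BeginPlay it binds to the player-name-changed event, sets the current name and gives the BP_PlayerNameTagUI widget a reference to itself.
; RefreshPlayerName reaches that widget through the BPPlayerNameTagActor's child WidgetComponent and sets its text.
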(event Custom|RefreshPlayerName
  (params (PlayerName :type String))
  (Rendering|Components|TextRender|SetText (Variables|/Game/Blueprints/UI/BP_PlayerNameTagUI.BP_PlayerNameTagUI_C|GetPlayerNameTag (.AsBP%20Player%20Name%20Tag%20UI (Utilities|Casting|CastToBP_PlayerNameTagUI (UserInterface|GetWidget (.As위젯%20컴포넌트 (Utilities|Casting|CastToWidgetComponent (Components|GetChildComponent (Variables|Default|GetBP_PlayerNameTagActor) 0))))))) (Utilities|Text|ToText(String) PlayerName)))

(event EventBeginPlay
  (EventDispatchers|BindEventtoOnPlayerNameChanged (EventDispatchers|CreateEvent :!event Custom|RefreshPlayerName))
  (CallFunction|RefreshPlayerName (Variables|Default|GetPlayerName))
  (Variables|/Game/Blueprints/UI/BP_PlayerNameTagUI.BP_PlayerNameTagUI_C|SetCompetitivePlayerCharacter (.AsBP%20Player%20Name%20Tag%20UI (Utilities|Casting|CastToBP_PlayerNameTagUI (UserInterface|GetWidget (.As위젯%20컴포넌트 (Utilities|Casting|CastToWidgetComponent (Components|GetChildComponent (Variables|Default|GetBP_PlayerNameTagActor) 0)))))) self))

(fn ConstructionScript)