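; BP_CompetitivePlayerController is a player controller that drives character movement and rotation from an on-screen virtual joystick.
; On BeginPlay, only for the local controller, it shows the mouse cursor, creates the joystick widget and adds it to the viewport.
; It binds two events to the widget, which pass the 2D input vectors to MoveWithVector2D and RotateWithVector2D, neither defined in this Blueprint.
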(event Custom|Player%20Controller%20Event
  (params (Vector%202D :type Vector%202D%20Structure))
  (Class|CompetitivePlayerController|MovewithVector2D Vector%202D))

(event Custom|Player%20Rotation%20Event
  (params (Vector%202D :type Vector%202D%20Structure))
  (Class|CompetitivePlayerController|RotatewithVector2D Vector%202D))

(event EventBeginPlay
  (if (Pawn|IsLocalPlayerController)
    (Variables|Default|SetbShowMouseCursor true)
    (bind _returnvalue (UserInterface|CreateWidget "/Game/Blueprints/UI/BP_VirtualJoystick.BP_VirtualJoystick_C"))
    (UserInterface|Viewport|AddtoViewport _returnvalue 0)
    (EventDispatchers|BindEventtoVirtualJoystick _returnvalue (delegate Custom|Player%20Controller%20Event))
    (EventDispatchers|BindEventtoCharacterRotation _returnvalue (delegate Custom|Player%20Rotation%20Event))))

(event EventTick
  (params (DeltaSeconds :type Float%20%28single-precision%29)))

(fn ConstructionScript)